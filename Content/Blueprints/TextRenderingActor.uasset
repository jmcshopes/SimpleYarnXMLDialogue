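; An NPC dialogue actor that shows greetings, responses and goodbyes on a TextRender component as an actor enters or leaves its overlap.
; Overlap creates the dialogue widget and toggles input and the mouse cursor for player controller 0.
; Answer events feed a branch tree keyed on dialogue state (UpdateArray) and choice, which sets the reply and next button texts.
; Only the first three states have responses, and the fourth answer calls an empty Leaving event.
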(event `self.ReceiveActorBeginOverlap`
  (params (OtherActor :type "Actor Object Reference"))
  (bind _returnvalue (`GameplayStatics.GetPlayerController` 0))
  ;[1 1 1] Start/End Encounter, Enable/disable input
  (`self.EnableInput` (`GameplayStatics.GetPlayerController` 0))
  (`TextRenderComponent.K2_SetText` (`self.TextRenderNPC1`) (`self.Greeting`))
  (bind _returnvalue_2 (`|CreateWidget` "/Game/Blueprints/DialogueWidget.DialogueWidget_C" _returnvalue))
  (`UserWidget.AddToViewport` _returnvalue_2 0)
  (bind _asplayer_controller (cast `PlayerController` _returnvalue))
  (set `PlayerController.bShowMouseCursor` true _asplayer_controller)
  (set `self.ButtonText` (`|MakeArray` (`self.Question 0-1`) (`self.Question 0-2`) (`self.Question 0-3`))))

(event `self.ReceiveActorEndOverlap`
  (params (OtherActor :type "Actor Object Reference"))
  ;[1 1 1] Start/End Encounter, Enable/disable input
  (`self.DisableInput` (`GameplayStatics.GetPlayerController` 0) null)
  (`TextRenderComponent.K2_SetText` (`self.TextRenderNPC1`) (`self.Goodbye`))
  (set `self.UpdateArray` 0)
  (`Widget.RemoveFromParent` (stale `self.ReceiveActorBeginOverlap` _returnvalue_2))
  (bind _asplayer_controller (cast `PlayerController` (`GameplayStatics.GetPlayerController` 0)))
  (set `PlayerController.bShowMouseCursor` false _asplayer_controller))

(event `Leaving`
  ;[1 1 1] Start/End Encounter, Enable/disable input
)

(event `Answer1`
  (bind _interact (`self.Interact`))
  (bind _interact_2 (`self.Interact`))
  (bind _interact_3 (`self.Interact`))
  (bind _array (`|MakeArray` (`self.Question 0-1`) (`self.Question 0-2`) (`self.Question 0-3`)))
  ;[1 1 1] Input
  (set `self.Interact` 0)
  ;[1 1 1] Question 1 Responses
  (if (== (`self.UpdateArray`) 0) :!label _label
    (if (== _interact_3 0)
      (`TextRenderComponent.K2_SetText` (`self.TextRenderNPC1`) (`self.Opt1Resp1`))
      (set `self.UpdateArray` 1)
      ;[1 1 1] Update UMG
      (set `self.ButtonText` (select `int` (`self.UpdateArray`) :`0` _array :`1` (`|MakeArray` (`self.Question 1-1`) (`self.Question 1-2`) (`self.Question 1-3`)) :`2` (`|MakeArray` (`self.Question 2-1`) (`self.Question 2-2`) (`self.Question 2-3`)) :`3` (`|MakeArray` (`self.Question 3-1`) (`self.Question 3-2`) (`self.Question 3-3`)) :`4` (`|MakeArray` (`self.Question 4-1`)) :`5` (`|MakeArray` (`self.Question 5-1`)) :`6` _array) :!label _label_2)
      (elif (== _interact_3 1)
        (`TextRenderComponent.K2_SetText` (`self.TextRenderNPC1`) (`self.Opt1Resp2`))
        (set `self.UpdateArray` 2)
        (goto _label_2)
        (elif (== _interact_3 2)
          (`TextRenderComponent.K2_SetText` (`self.TextRenderNPC1`) (`self.Opt1Resp3`))
          (set `self.UpdateArray` 3)
          (goto _label_2))))
    (else
      ;[1 1 1] Question 2 Responses
      (if (== (`self.UpdateArray`) 1)
        (if (== _interact 0)
          (`TextRenderComponent.K2_SetText` (`self.TextRenderNPC1`) (`self.Opt2Resp1`))
          (set `self.UpdateArray` 2)
          (goto _label_2)
          (elif (== _interact 1)
            (`TextRenderComponent.K2_SetText` (`self.TextRenderNPC1`) (`self.Opt2Resp2`))
            (set `self.UpdateArray` 3)
            (goto _label_2)
            (elif (== _interact 2)
              (`TextRenderComponent.K2_SetText` (`self.TextRenderNPC1`) (`self.Opt2Resp3`))
              (set `self.UpdateArray` 6)
              (goto _label_2))))
        (else
          ;[1 1 1] Question 3 Responses
          (if (== (`self.UpdateArray`) 2)
            (if (== _interact_2 0)
              (`TextRenderComponent.K2_SetText` (`self.TextRenderNPC1`) (`self.Op3Resp1`))
              (set `self.UpdateArray` 1)
              (goto _label_2)
              (elif (== _interact_2 1)
                (`TextRenderComponent.K2_SetText` (`self.TextRenderNPC1`) (`self.Opt3Resp2`))
                (set `self.UpdateArray` 2)
                (goto _label_2)
                (elif (== _interact_2 2)
                  (`TextRenderComponent.K2_SetText` (`self.TextRenderNPC1`) (`self.Opt3Resp3`))
                  (set `self.UpdateArray` 6)
                  (goto _label_2))))))))))

(event `Answer2`
  ;[1 1 1] Input
  (set `self.Interact` 1)
  (goto _label))

(event `Answer3`
  ;[1 1 1] Input
  (set `self.Interact` 2)
  (goto _label))

(event `Answer4`
  ;[1 1 1] Leaving Now Response
  (`self.Leaving`))

(fn `UserConstructionScript`)