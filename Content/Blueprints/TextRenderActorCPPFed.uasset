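; NPC dialogue actor that starts an encounter on overlap, disabling player input and showing a dialogue widget with the mouse cursor.
; DialogueGetter looks up the next nodes for NPCName from the current node, starting at "Start", to refill the button text and node arrays.
; The first three answer events advance to their stored node.
; The fourth answer or ending overlap closes the widget and restores input.
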(event `self.ReceiveActorBeginOverlap`
  (params (OtherActor :type "Actor Object Reference"))
  (bind _returnvalue (`GameplayStatics.GetPlayerController` 0))
  ;[1 1 1] Start/End Encounter, Enable/disable input
  (`self.DisableInput` (`GameplayStatics.GetPlayerController` 0) null)
  (bind _returnvalue_2 (`|CreateWidget` "/Game/Blueprints/DialogueWidget.DialogueWidget_C" _returnvalue))
  (`UserWidget.AddToViewport` _returnvalue_2 0)
  (set `PlayerController.bShowMouseCursor` true _returnvalue)
  (bind _output_get (set `DialogueGetter.CurrentNode` "Start" (`self.DialogueGetter`)))
  (bind _returnvalue_3 (`DialogueGetter.GetNextNode` (`self.DialogueGetter`) _output_get (`self.NPCName`) :!label _label))
  (`KismetArrayLibrary.Array_Clear` (`self.ButtonText`))
  (`KismetArrayLibrary.Array_Clear` (`self.Nodes`))
  (for _array_element _returnvalue_3
    (bind (_index _option _optioncode _node) (break `PlayerOptionType` _array_element))
    (`KismetArrayLibrary.Array_Add` (`self.Nodes`) _node)
    (`KismetArrayLibrary.Array_Add` (`self.ButtonText`) (`KismetTextLibrary.Conv_StringToText` _option))))

(event `self.ReceiveActorEndOverlap`
  (params (OtherActor :type "Actor Object Reference"))
  ;[1 1 1] Start/End Encounter, Enable/disable input
  (`self.EnableInput` (`GameplayStatics.GetPlayerController` 0) null :!label _label_2)
  (set `self.UpdateArray` 0)
  (`Widget.RemoveFromParent` (stale `self.ReceiveActorBeginOverlap` _returnvalue_2))
  (set `PlayerController.bShowMouseCursor` false (`GameplayStatics.GetPlayerController` 0)))

(event `Leaving`
  ;[1 1 1] Start/End Encounter, Enable/disable input
  (goto _label_2))

(event `Answer1`
  ;[1 1 1] Input
  (set `self.Interact` 0)
  (set `DialogueGetter.CurrentNode` (`|GetArrayItem` (`self.Nodes`) (`self.Interact`)) (`self.DialogueGetter`) :!label _label_3)
  (goto _label))

(event `Answer2`
  ;[1 1 1] Input
  (set `self.Interact` 1)
  (goto _label_3))

(event `Answer3`
  ;[1 1 1] Input
  (set `self.Interact` 2)
  (goto _label_3))

(event `Answer4`
  ;[1 1 1] Leaving Now Response
  (`self.Leaving`))

(fn `UserConstructionScript`)